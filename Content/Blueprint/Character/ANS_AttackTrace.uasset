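; ANS_AttackTrace is an anim notify state that drives sword hit detection during attack animations for BP_IroncladCharacter.
; Each notify tick casts the mesh owner to that character and calls DoTrace on its Sword.
; When the notify window ends, it clears the Sword's HitActors list, resetting the recorded hits from that swing.
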(fn `Received_NotifyEnd`
  (params (MeshComp :type "SkeletalMeshComponent Object Reference") (Animation :type "AnimSequenceBase Object Reference") (EventReference :type "AnimNotifyEventReference Structure (by ref)"))
  (returns (ReturnValue :type Boolean))
  (bind _asbp_ironclad_character (cast `/Game/Blueprint/Character/BP_IroncladCharacter` (`ActorComponent.GetOwner` MeshComp)))
  (`KismetArrayLibrary.Array_Clear` (`/Game/Blueprint/Character/BP_Sword.HitActors` (`/Game/Blueprint/Character/BP_IroncladCharacter.Sword` _asbp_ironclad_character)))
  (return false))

(fn `Received_NotifyTick`
  (params (MeshComp :type "SkeletalMeshComponent Object Reference") (Animation :type "AnimSequenceBase Object Reference") (FrameDeltaTime :type "Float (single-precision)") (EventReference :type "AnimNotifyEventReference Structure (by ref)"))
  (returns (ReturnValue :type Boolean))
  (bind _asbp_ironclad_character (cast `/Game/Blueprint/Character/BP_IroncladCharacter` (`ActorComponent.GetOwner` MeshComp)))
  (`/Game/Blueprint/Character/BP_Sword.DoTrace` (`/Game/Blueprint/Character/BP_IroncladCharacter.Sword` _asbp_ironclad_character))
  (return false))