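; BP_Enemy is an enemy character that senses the player through AI Perception and drives its AI through blackboard keys.
; Sensing a Player-tagged actor stores it as the blackboard target and changes state unless that Ironclad character is in a particular state; other perception updates clear the target and switch state.
; UpdateState writes state and attack range to the blackboard, with one state locking out further changes.
; UpdateSpeed sets maximum walk speed.
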(event `UpdateState`
  (params (NewState :type "/Game/Blueprint/Monster/EEnemyState Enum" :default "NewEnumerator3"))
  (bind _returnvalue (`AIBlueprintHelperLibrary.GetBlackboard` (`AIBlueprintHelperLibrary.GetAIController` self)))
  (if (`|EnumInequality` (`self.State`) "NewEnumerator4")
    (bind _output_get (set `self.State` NewState))
    (`BlackboardComponent.SetValueAsEnum` _returnvalue (`self.StateKey`) _output_get)
    (`BlackboardComponent.SetValueAsFloat` _returnvalue (`self.AttackRangeKey`) (`self.AttackRange`))))

(event `self.AIPerception.OnTargetPerceptionUpdated`
  (params (Actor :type "Actor Object Reference") (Stimulus :type "AIStimulus Structure"))
  ; 적 감지
  (if (and (`self.ActorHasTag` Actor "Player") (`.bSuccessfullySensed` (break `AIStimulus` Stimulus)))
    (`BlackboardComponent.SetValueAsObject` (`AIController.Blackboard` (`AIBlueprintHelperLibrary.GetAIController` self)) (`self.EnemyActorKey`) Actor)
    (bind _asbp_ironclad_character (cast `/Game/Blueprint/Character/BP_IroncladCharacter` Actor))
    (if (not (`|EnumEquality` (`/Game/Blueprint/Character/BP_IroncladCharacter.State` _asbp_ironclad_character) "NewEnumerator3"))
      (`self.UpdateState` "NewEnumerator1"))
    (else
      (`BlackboardComponent.ClearValue` (`AIBlueprintHelperLibrary.GetBlackboard` (`AIBlueprintHelperLibrary.GetAIController` self)) (`self.EnemyActorKey`))
      (`self.UpdateState` "NewEnumerator3"))))

(fn `UpdateSpeed`
  (params (NewSpeed :type "Float (double-precision)"))
  (set `CharacterMovementComponent.MaxWalkSpeed` NewSpeed (`self.CharacterMovement`)))

(fn `UserConstructionScript`)