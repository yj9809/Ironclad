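; Base enemy character that takes damage, reacts to hits and dissolves on death.
; AnyDamage feeds the health component, whose HP-change event plays a hit montage except in one specific state.
; Its death event sets the state, disables capsule collision, passes the state to BP_EnemyController, then after a delay runs a material Dissolve timeline and destroys the actor.
; UpdateSpeed exposes walk speed changes.
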(event `self.ReceiveBeginPlay`
  (bind _bp_healthcomponent (`self.BP_HealthComponent`))
  (set `self.CurrentHP` (`self.MaxHP`))
  (add `/Game/Blueprint/BP_HealthComponent.OnDead` _bp_healthcomponent (delegate `OnDead`))
  (add `/Game/Blueprint/BP_HealthComponent.OnHPCanged` _bp_healthcomponent (delegate `OnHPChanged`))
  (`/Game/Blueprint/BP_HealthComponent.UpdateHP` (`self.BP_HealthComponent`) (`self.MaxHP`)))

(event `OnHPChanged`
  (params (CurrentHP :type "Float (double-precision)") (MaxHP :type "Float (double-precision)"))
  (if (`|EnumInequality` (`self.State`) "NewEnumerator2")
    (`|PlayMontage` (`self.Mesh`) (`self.HitMontage`))))

(event `OnDead`
  (bind _output_get (set `self.State` "NewEnumerator4"))
  (`PrimitiveComponent.SetCollisionEnabled` (`self.CapsuleComponent`) "NoCollision")
  (bind _asbp_enemy_controller (cast `/Game/Blueprint/Monster/BP_EnemyController` (`self.GetController` self)))
  (`/Game/Blueprint/Monster/BP_EnemyController.UpdateState` _asbp_enemy_controller _output_get)
  (`KismetSystemLibrary.Delay` 2.0)
  (bind (_direction _dissolve) (`Timeline|DeadEffect` :!via `PlayFromStart`)
    (:`Update`
      (`MeshComponent.SetScalarParameterValueOnMaterials` (`self.Mesh`) "Dissolve" _dissolve))
    (:`Finished`
      (`self.K2_DestroyActor`))))

(event `self.ReceiveAnyDamage`
  (params (Damage :type "Float (single-precision)") (DamageType :type "DamageType Object Reference") (InstigatedBy :type "Controller Object Reference") (DamageCauser :type "Actor Object Reference"))
  (`/Game/Blueprint/BP_HealthComponent.ReceiveDamage` (`self.BP_HealthComponent`) Damage))

(fn `UpdateSpeed`
  (params (NewSpeed :type "Float (double-precision)"))
  (set `CharacterMovementComponent.MaxWalkSpeed` NewSpeed (`self.CharacterMovement`)))

(fn `UserConstructionScript`)