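; BP_Enemy is a monster character that attacks BP_IroncladCharacter, reacts to hits and dissolves on death.
; BPHealthComponent takes incoming damage and drives hit montages and death, which updates BP_EnemyController and runs a dissolve timeline before destroy.
; Left and right attack overlaps spawn blood and share one ApplyDamage, targeting the right-hand cast result.
; Tick caps height, while helper functions set walk speed and reset gravity and Blackboard state after launches.
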(event `self.ReceiveBeginPlay`
  (`|ExecutionSequence`
    (:`then_0`
      ; 데미지/죽음 이벤트 등록
      (add `/Game/Blueprint/BP_HealthComponent.OnDead` (`self.BP_HealthComponent`) (delegate `OnDead`))
      (add `/Game/Blueprint/BP_HealthComponent.OnHPCanged` (`self.BP_HealthComponent`) (delegate `OnHPChanged`))
      (`/Game/Blueprint/BP_HealthComponent.UpdateHP` (`self.BP_HealthComponent`) (`self.MaxHP`)))
    (:`then_1`
      ; Attack Collision On/Off
      (`PrimitiveComponent.SetCollisionEnabled` (`self.AttackCollision_l`) "NoCollision")
      (`PrimitiveComponent.SetCollisionEnabled` (`self.AttackCollision_r`) "NoCollision"))))

(event `OnHPChanged`
  (params (CurrentHP :type "Float (double-precision)") (MaxHP :type "Float (double-precision)"))
  ; 데미지/죽음 이벤트 등록
  (set `self.CurrentHP` CurrentHP)
  (if (`|EnumInequality` (`self.State`) "NewEnumerator2")
    (`|PlayMontage` (`self.Mesh`) "/Game/Blueprint/Monster/WhisperActor/AM_EnemyHit.AM_EnemyHit")))

(event `OnDead`
  ; 데미지/죽음 이벤트 등록
  (bind _output_get (set `self.State` "NewEnumerator4"))
  (`PrimitiveComponent.SetCollisionEnabled` (`self.CapsuleComponent`) "NoCollision")
  (bind _asbp_enemy_controller (cast `/Game/Blueprint/Monster/BP_EnemyController` (`self.GetController` self)))
  (`/Game/Blueprint/Monster/BP_EnemyController.UpdateState` _asbp_enemy_controller _output_get)
  (`KismetSystemLibrary.Delay` 2.0)
  (bind (_direction _dissolve) (`Timeline|DeadEffect` :!via `PlayFromStart`)
    (:`Update`
      (`MeshComponent.SetScalarParameterValueOnMaterials` (`self.Mesh`) "Dissolve" _dissolve))
    (:`Finished`
      (`self.K2_DestroyActor`))))

(event `self.ReceiveAnyDamage`
  (params (Damage :type "Float (single-precision)") (DamageType :type "DamageType Object Reference") (InstigatedBy :type "Controller Object Reference") (DamageCauser :type "Actor Object Reference"))
  ; 히트 이펙트 처리
  (`/Game/Blueprint/BP_HealthComponent.ReceiveDamage` (`self.BP_HealthComponent`) Damage))

(event `self.AttackCollision_l.OnComponentBeginOverlap`
  (params (OverlappedComponent :type "PrimitiveComponent Object Reference") (OtherActor :type "Actor Object Reference") (OtherComp :type "PrimitiveComponent Object Reference") (OtherBodyIndex :type Integer) (bFromSweep :type Boolean) (SweepResult :type "HitResult Structure (by ref)"))
  ; 몬스터 공격 처리
  (bind _asbp_ironclad_character (cast `/Game/Blueprint/Character/BP_IroncladCharacter` OtherActor))
  (`NiagaraFunctionLibrary.SpawnSystemAtLocation` "/Game/Effect/NS_Blood_VFX.NS_Blood_VFX" (`self.K2_GetActorLocation` _asbp_ironclad_character) (`KismetMathLibrary.RandomRotator` false))
  (`GameplayStatics.ApplyDamage` (stale `self.AttackCollision_r.OnComponentBeginOverlap` _asbp_ironclad_character) (`self.Damage`) null self :!label _label))

(event `self.ReceiveTick`
  (params (DeltaSeconds :type "Float (single-precision)"))
  (bind (_returnvalue_x _returnvalue_y _returnvalue_z) (`KismetMathLibrary.BreakVector` (`self.K2_GetActorLocation`)))
  (`self.K2_SetActorLocation` (`KismetMathLibrary.MakeVector` _returnvalue_x _returnvalue_y (`KismetMathLibrary.FClamp` _returnvalue_z -9999.0 450.0))))

(event `self.AttackCollision_r.OnComponentBeginOverlap`
  (params (OverlappedComponent :type "PrimitiveComponent Object Reference") (OtherActor :type "Actor Object Reference") (OtherComp :type "PrimitiveComponent Object Reference") (OtherBodyIndex :type Integer) (bFromSweep :type Boolean) (SweepResult :type "HitResult Structure (by ref)"))
  ; 몬스터 공격 처리
  (bind _asbp_ironclad_character (cast `/Game/Blueprint/Character/BP_IroncladCharacter` OtherActor))
  (`NiagaraFunctionLibrary.SpawnSystemAtLocation` "/Game/Effect/NS_Blood_VFX.NS_Blood_VFX" (`self.K2_GetActorLocation` _asbp_ironclad_character) (`KismetMathLibrary.RandomRotator` false))
  (goto _label))

(fn `ResetLaunchFuntion`
  (set `CharacterMovementComponent.GravityScale` 5.0 (`self.CharacterMovement`))
  (bind _output_get (set `self.State` "NewEnumerator1"))
  (`BlackboardComponent.SetValueAsEnum` (`AIBlueprintHelperLibrary.GetBlackboard` (`AIBlueprintHelperLibrary.GetAIController` self)) (`self.StateKey`) _output_get))

(fn `UpdateSpeed`
  (params (NewSpeed :type "Float (double-precision)"))
  (set `CharacterMovementComponent.MaxWalkSpeed` NewSpeed (`self.CharacterMovement`)))

(fn `UserConstructionScript`)