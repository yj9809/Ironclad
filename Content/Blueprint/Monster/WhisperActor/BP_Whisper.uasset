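; BP_Whisper is a monster whose left and right attack colliders damage the Ironclad character.
; Both colliders start disabled; each overlap spawns blood VFX and feeds a shared ApplyDamage node, which targets only the right handler's cast result.
; Tick caps the monster's height.
; ResetLaunchFuntion sets gravity scale and writes the AI blackboard state key, apparently to recover from a launch.
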(event `self.ReceiveBeginPlay`
  (`parent.ReceiveBeginPlay`)
  (`|ExecutionSequence`
    (:`then_1`
      ; Attack Collision On/Off
      (`PrimitiveComponent.SetCollisionEnabled` (`self.AttackCollision_l`) "NoCollision")
      (`PrimitiveComponent.SetCollisionEnabled` (`self.AttackCollision_r`) "NoCollision"))))

(event `self.AttackCollision_l.OnComponentBeginOverlap`
  (params (OverlappedComponent :type "PrimitiveComponent Object Reference") (OtherActor :type "Actor Object Reference") (OtherComp :type "PrimitiveComponent Object Reference") (OtherBodyIndex :type Integer) (bFromSweep :type Boolean) (SweepResult :type "HitResult Structure (by ref)"))
  ; 몬스터 공격 처리
  (bind _asbp_ironclad_character (cast `/Game/Blueprint/Character/BP_IroncladCharacter` OtherActor))
  (`NiagaraFunctionLibrary.SpawnSystemAtLocation` "/Game/Effect/NS_Blood_VFX.NS_Blood_VFX" (`self.K2_GetActorLocation` _asbp_ironclad_character) (`KismetMathLibrary.RandomRotator` false))
  (`GameplayStatics.ApplyDamage` (stale `self.AttackCollision_r.OnComponentBeginOverlap` _asbp_ironclad_character) (`self.Damage`) null self :!label _label))

(event `self.ReceiveTick`
  (params (DeltaSeconds :type "Float (single-precision)"))
  (bind (_returnvalue_x _returnvalue_y _returnvalue_z) (`KismetMathLibrary.BreakVector` (`self.K2_GetActorLocation`)))
  (`self.K2_SetActorLocation` (`KismetMathLibrary.MakeVector` _returnvalue_x _returnvalue_y (`KismetMathLibrary.FClamp` _returnvalue_z -9999.0 450.0))))

(event `self.AttackCollision_r.OnComponentBeginOverlap`
  (params (OverlappedComponent :type "PrimitiveComponent Object Reference") (OtherActor :type "Actor Object Reference") (OtherComp :type "PrimitiveComponent Object Reference") (OtherBodyIndex :type Integer) (bFromSweep :type Boolean) (SweepResult :type "HitResult Structure (by ref)"))
  ; 몬스터 공격 처리
  (bind _asbp_ironclad_character (cast `/Game/Blueprint/Character/BP_IroncladCharacter` OtherActor))
  (`NiagaraFunctionLibrary.SpawnSystemAtLocation` "/Game/Effect/NS_Blood_VFX.NS_Blood_VFX" (`self.K2_GetActorLocation` _asbp_ironclad_character) (`KismetMathLibrary.RandomRotator` false))
  (goto _label))

(fn `ResetLaunchFuntion`
  (set `CharacterMovementComponent.GravityScale` 5.0 (`self.CharacterMovement`))
  (`BlackboardComponent.SetValueAsEnum` (`AIBlueprintHelperLibrary.GetBlackboard` (`AIBlueprintHelperLibrary.GetAIController` self)) (`self.StateKey`) 0))

(fn `UserConstructionScript`)