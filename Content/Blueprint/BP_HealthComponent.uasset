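; BP_HealthComponent is a health component that tracks current and maximum HP and signals damage and death.
; It fills HP to maximum on BeginPlay, and UpdateHP sets a new maximum and refills without broadcasting.
; ReceiveDamage subtracts damage only while HP is positive, then calls the OnHPCanged dispatcher.
; When HP reaches zero or below it calls OnDead, with no clamping of the value.
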(event `UpdateHP`
  (params (MaxHP :type "Float (double-precision)"))
  ; HP 업데이트
  (bind _output_get (set `self.MaxHP` MaxHP))
  (set `self.CurrentHP` _output_get))

(event `self.ReceiveBeginPlay`
  ; 시작 HP 설정
  (set `self.CurrentHP` (`self.MaxHP`)))

(event `ReceiveDamage`
  (params (Damage :type "Float (double-precision)"))
  ; Damage 처리
  (if (> (`self.CurrentHP`) 0.0)
    (bind _output_get (set `self.CurrentHP` (- (`self.CurrentHP`) Damage)))
    (`self.OnHPCanged` _output_get (`self.MaxHP`) Damage)
    (if (<= _output_get 0.0)
      (`self.OnDead`))))