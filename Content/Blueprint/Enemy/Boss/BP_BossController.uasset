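; AI controller for the boss enemy that drives its health-based phase change.
; On possess it caches the BP_Boss pawn, and on begin play it sets NeverLoseTarget.
; Every tick it compares current HP to half of max and writes the phase flag to the Blackboard.
; At or below half health it also raises the boss's play rate and walk speed, reapplying both each tick.
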(event `self.ReceivePossess`
  (params (PossessedPawn :type "Pawn Object Reference"))
  (bind _asbp_boss (cast `/Game/Blueprint/Enemy/Boss/BP_Boss` PossessedPawn))
  (set `self.BossPawn` _asbp_boss)
  (`parent.ReceivePossess` PossessedPawn))

(event `self.ReceiveBeginPlay`
  (set `self.NeverLoseTarget` true))

(event `self.ReceiveTick`
  (params (DeltaSeconds :type "Float (single-precision)"))
  (bind _bosspawn (`self.BossPawn`))
  (bind _phasekey (`self.PhaseKey`))
  (bind _returnvalue (`AIBlueprintHelperLibrary.GetBlackboard` (`AIBlueprintHelperLibrary.GetAIController` (`self.BossPawn`))))
  (if (> (`/Game/Blueprint/Enemy/BP_EnemyBase.CurrentHP` _bosspawn) (/ (`/Game/Blueprint/Enemy/BP_EnemyBase.MaxHP` _bosspawn) 2.0))
    (`BlackboardComponent.SetValueAsBool` _returnvalue _phasekey false)
    (else
      (`BlackboardComponent.SetValueAsBool` _returnvalue _phasekey true)
      (set `/Game/Blueprint/Enemy/Boss/BP_Boss.BossPlayRate` 2.0 _bosspawn)
      (set `CharacterMovementComponent.MaxWalkSpeed` 800.0 (`Character.CharacterMovement` _bosspawn)))))

(fn `UserConstructionScript`)