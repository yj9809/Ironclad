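; Whisper enemy Blueprint that sets up its hit and attack montages, attack colliders and the shared enemy behavior tree and blackboard on top of parent logic.
; Left and right attack collision overlaps apply damage and spawn blood VFX on the Ironclad character.
; HP changes briefly show the overhead health widget, which stays visible while locked on.
; Tick caps world height, and a launch reset function sets gravity and blackboard state.
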(event `self.ReceiveBeginPlay`
  (bind _returnvalue (`WidgetComponent.GetUserWidgetObject` (`self.EnemyHP`)))
  (`self.Init`)
  (`parent.ReceiveBeginPlay`)
  (bind _aswbp_enemy_hp (cast `/Game/Blueprint/UI/WBP_EnemyHP` _returnvalue))
  (set `/Game/Blueprint/UI/WBP_EnemyHP.EnemyReference` self _aswbp_enemy_hp)
  (`Widget.SetVisibility` _returnvalue "Hidden")
  (set `self.HitMontage` "/Game/Blueprint/Enemy/WhisperActor/AM_WhisperHit.AM_WhisperHit")
  (set `self.AttackMontage` "/Game/Blueprint/Enemy/WhisperActor/AM_WhisperAttack.AM_WhisperAttack"))

(event `self.OnHPChanged`
  (params (CurrentHP :type "Float (double-precision)") (MaxHP :type "Float (double-precision)") (Damage :type "Float (double-precision)"))
  ; 데미지 처리 시 UI 표시
  (`parent.OnHPChanged` CurrentHP MaxHP Damage)
  (bind _aswbp_enemy_hp (`self.HpUiVisibility` true))
  (`/Game/Blueprint/UI/WBP_EnemyHP.HpChange` _aswbp_enemy_hp CurrentHP)
  (`KismetSystemLibrary.K2_SetTimerDelegate` (delegate `HpUiOff`) 1.0))

(event `HpUiOff`
  ; 데미지 처리 시 UI 표시
  (if (not (`self.IsLockOn`))
    (`self.HpUiVisibility` false)))

(event `self.AttackCollision_l.OnComponentBeginOverlap`
  (params (OverlappedComponent :type "PrimitiveComponent Object Reference") (OtherActor :type "Actor Object Reference") (OtherComp :type "PrimitiveComponent Object Reference") (OtherBodyIndex :type Integer) (bFromSweep :type Boolean) (SweepResult :type "HitResult Structure (by ref)"))
  ; 몬스터 공격 처리
  (bind _asbp_ironclad_character (cast `/Game/Blueprint/Character/BP_IroncladCharacter` OtherActor))
  (`NiagaraFunctionLibrary.SpawnSystemAtLocation` "/Game/Effect/NS_Blood_VFX.NS_Blood_VFX" (`self.K2_GetActorLocation` _asbp_ironclad_character) (`KismetMathLibrary.RandomRotator` false))
  (`GameplayStatics.ApplyDamage` _asbp_ironclad_character (`self.Damage`) null self))

(event `self.ReceiveTick`
  (params (DeltaSeconds :type "Float (single-precision)"))
  (bind (_returnvalue_x _returnvalue_y _returnvalue_z) (`KismetMathLibrary.BreakVector` (`self.K2_GetActorLocation`)))
  (`self.K2_SetActorLocation` (`KismetMathLibrary.MakeVector` _returnvalue_x _returnvalue_y (`KismetMathLibrary.FClamp` _returnvalue_z -9999.0 450.0))))

(event `self.AttackCollision_r_0.OnComponentBeginOverlap`
  (params (OverlappedComponent :type "PrimitiveComponent Object Reference") (OtherActor :type "Actor Object Reference") (OtherComp :type "PrimitiveComponent Object Reference") (OtherBodyIndex :type Integer) (bFromSweep :type Boolean) (SweepResult :type "HitResult Structure (by ref)"))
  ; 몬스터 공격 처리
  (bind _asbp_ironclad_character (cast `/Game/Blueprint/Character/BP_IroncladCharacter` OtherActor))
  (`NiagaraFunctionLibrary.SpawnSystemAtLocation` "/Game/Effect/NS_Blood_VFX.NS_Blood_VFX" (`self.K2_GetActorLocation` _asbp_ironclad_character) (`KismetMathLibrary.RandomRotator` false))
  (`GameplayStatics.ApplyDamage` _asbp_ironclad_character (`self.Damage`) null self))

(fn `HpUiVisibility`
  (params (Visibility :type Boolean))
  (returns (`AsWBP Enemy HP` :type "/Game/Blueprint/UI/WBP_EnemyHP Object Reference"))
  (bind _returnvalue (`WidgetComponent.GetUserWidgetObject` (`self.EnemyHP`)))
  (if Visibility
    (`Widget.SetVisibility` _returnvalue "Visible")
    (bind _aswbp_enemy_hp (cast `/Game/Blueprint/UI/WBP_EnemyHP` _returnvalue))
    (return _aswbp_enemy_hp)
    (else
      (`Widget.SetVisibility` _returnvalue "Hidden"))))

(fn `Init`
  (set `self.AttackCollsion_l` (`self.AttackCollision_l`))
  (set `self.AttackCollision_r` (`self.AttackCollision_r_0`))
  (set `self.CurrentBB` "/Game/Blueprint/Enemy/AI/BB_Enemy.BB_Enemy")
  (set `self.CurrentBT` "/Game/Blueprint/Enemy/AI/BT_Enemy.BT_Enemy"))

(fn `ResetLaunchFuntion`
  (set `CharacterMovementComponent.GravityScale` 5.0 (`self.CharacterMovement`))
  (`BlackboardComponent.SetValueAsEnum` (`AIBlueprintHelperLibrary.GetBlackboard` (`AIBlueprintHelperLibrary.GetAIController` self)) (`self.StateKey_0`) 0))

(fn `UserConstructionScript`)