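; AI controller for BP_EnemyBase enemies that runs each pawn's own Behavior Tree and Blackboard, seeding home location and attack range on possess.
; Perceiving the player sets the target and, depending on player state, switches enemy state, speeds it up and creates a boss HUD for bosses.
; Losing sight reverts these after a delay, unless NeverLoseTarget is set.
; UpdateState mirrors state to pawn and Blackboard, with one state locking the controller's copy.
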(event `self.ReceivePossess`
  (params (PossessedPawn :type "Pawn Object Reference"))
  (bind _returnvalue (`AIBlueprintHelperLibrary.GetBlackboard` null))
  (bind _asbp_enemy_base (cast `/Game/Blueprint/Enemy/BP_EnemyBase` PossessedPawn))
  (`|ExecutionSequence`
    (:`then_0`
      (`self.UseBlackboard` (`/Game/Blueprint/Enemy/BP_EnemyBase.CurrentBB` _asbp_enemy_base))
      (`self.RunBehaviorTree` (`/Game/Blueprint/Enemy/BP_EnemyBase.CurrentBT` _asbp_enemy_base))
      (bind _asbp_enemy_base_2 (cast `/Game/Blueprint/Enemy/BP_EnemyBase` (`self.K2_GetPawn`)))
      (set `self.EnemyActor` _asbp_enemy_base_2))
    (:`then_1`
      (`BlackboardComponent.SetValueAsVector` _returnvalue (`self.HomeLocationKey`) (`self.K2_GetActorLocation` PossessedPawn))
      (`BlackboardComponent.SetValueAsFloat` _returnvalue (`self.AttackRangeKey`) 50.0))))

(event `self.AIPerception.OnTargetPerceptionUpdated`
  (params (Actor :type "Actor Object Reference") (Stimulus :type "AIStimulus Structure"))
  ; AI 감지
  (if (`.bSuccessfullySensed` (break `AIStimulus` Stimulus))
    (if (`|EnumInequality` (`self.State`) "NewEnumerator4")
      (if (`self.ActorHasTag` Actor "Player")
        (set `self.LostSight` false)
        (`BlackboardComponent.SetValueAsObject` (`self.Blackboard`) (`self.EnemyActorKey`) Actor)
        (bind _asbp_ironclad_character (cast `/Game/Blueprint/Character/BP_IroncladCharacter` Actor))
        (if (not (`|EnumEquality` (`/Game/Blueprint/Character/BP_IroncladCharacter.State` _asbp_ironclad_character) "NewEnumerator3"))
          (`self.UpdateState` "NewEnumerator1")
          (set `self.State` "NewEnumerator1")
          (`self.UpdateSpeed` 400.0)
          ;; 보스 몬스터일 경우 HP UI 표시
          (bind _asbp_boss (cast `/Game/Blueprint/Enemy/Boss/BP_Boss` (`self.K2_GetPawn`)))
          (bind _returnvalue (`|CreateWidget` "/Game/Blueprint/UI/WBP_BossHUD.WBP_BossHUD_C"))
          (set `/Game/Blueprint/UI/WBP_BossHUD.Boss Reference` _asbp_boss _returnvalue)
          (set `/Game/Blueprint/Enemy/Boss/BP_Boss.HpHUD` _returnvalue _asbp_boss)
          (`UserWidget.AddToViewport` _returnvalue 0))))
    (elif (not (`self.NeverLoseTarget`))
      (set `self.LostSight` true)
      (if (`self.ActorHasTag` Actor "Player")
        (`KismetSystemLibrary.Delay` 3.0)
        (if (`self.LostSight`)
          (`BlackboardComponent.ClearValue` (`AIBlueprintHelperLibrary.GetBlackboard` self) (`self.EnemyActorKey`))
          (`self.UpdateState` "NewEnumerator0")
          (set `self.State` "NewEnumerator0")
          (`self.UpdateSpeed` 200.0))))))

(event `UpdateState`
  (params (NewState :type "/Game/Blueprint/Enemy/EEnemyState Enum" :default "NewEnumerator3"))
  (bind _attackrangekey (`self.AttackRangeKey`))
  (bind _returnvalue (`AIBlueprintHelperLibrary.GetBlackboard` self))
  ; Enemy 상태 업데이트
  (if (`|EnumInequality` (`self.State`) "NewEnumerator4")
    (bind _output_get (set `self.State` NewState))
    (bind _asbp_enemy_base (cast `/Game/Blueprint/Enemy/BP_EnemyBase` (`self.K2_GetPawn` self)))
    (set `/Game/Blueprint/Enemy/BP_EnemyBase.State` _output_get _asbp_enemy_base)
    (`BlackboardComponent.SetValueAsEnum` _returnvalue (`self.StateKey`) _output_get)
    (`BlackboardComponent.SetValueAsFloat` _returnvalue _attackrangekey (`BlackboardComponent.GetValueAsFloat` (`AIBlueprintHelperLibrary.GetBlackboard` self) _attackrangekey))
    (else
      (`BlackboardComponent.SetValueAsEnum` (`AIBlueprintHelperLibrary.GetBlackboard` self) (`self.StateKey`) NewState))))

(fn `UpdateSpeed`
  (params (NewSpeed :type "Float (double-precision)"))
  (bind _asbp_enemy_base (cast `/Game/Blueprint/Enemy/BP_EnemyBase` (`self.K2_GetPawn`)))
  (set `CharacterMovementComponent.MaxWalkSpeed` NewSpeed (`Character.CharacterMovement` _asbp_enemy_base)))

(fn `UserConstructionScript`)